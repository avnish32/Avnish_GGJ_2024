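; BP_Container is an interactable deposit point for punchlines, tied to a joke shown on a decal.
; On begin play it caches the HUD and player, then puts a dynamic material with the question texture on TextDecal.
; Interacting with a non-empty inventory opens the HUD's interactive inventory and pauses the game with a cursor.
; A correct punchline swaps the decal to the answer texture and destroys the container.
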(event Custom|OnCorrectPunchline
  (Rendering|Material|SetTextureParameterValue (Variables|Default|GetjokeTextMaterial) "Texture" (Variables|Default|GetanswerTexture))
  (Actor|DestroyActor))

(event EventBeginPlay
  (bind _returnvalue (Actor|GetActorOfClass "/Game/UI/HUD/BP_HUD.BP_HUD_C"))
  (Variables|Default|Sethud _returnvalue)
  (bind _returnvalue_2 (Actor|GetActorOfClass "/Game/FirstPerson/Blueprints/BP_FirstPersonCharacter.BP_FirstPersonCharacter_C"))
  (Variables|Default|SetFPC _returnvalue_2)
  (bind _returnvalue_3 (Rendering|Material|CreateDynamicMaterialInstance "/Game/Materials/Texts/MI_JokeText.MI_JokeText" "None" "None" :!class /Script/Engine.KismetMaterialLibrary))
  (bind _output_get (Variables|Default|SetjokeTextMaterial _returnvalue_3))
  (Rendering|Material|SetTextureParameterValue _output_get "Texture" (Variables|Default|GetquestionTexture))
  (Rendering|Components|Decal|SetDecalMaterial (Variables|/Script/Engine.DecalActor|GetDecal (Variables|Default|GettextDecal)) (Variables|Default|GetjokeTextMaterial)))

(event Collision|EventActorBeginOverlap
  (params (OtherActor :type Actor%20Object%20Reference)))

(event EventTick
  (params (DeltaSeconds :type Float%20%28single-precision%29)))

(event EventDisplayInteractMsg
  (bind _hud (Variables|Default|Gethud))
  (if (Utilities|Array|IsEmpty (Variables|/Game/FirstPerson/Blueprints/BP_FirstPersonCharacter.BP_FirstPersonCharacter_C|Getinventory (Variables|Default|GetFPC)))
    (Default|DisplayRaycastMsg _hud "No punchlines to deposit")
    (else
      (Default|DisplayRaycastMsg _hud "Deposit"))))

(event EventInteract
  (bind _hud (Variables|Default|Gethud))
  (if (not (Utilities|Array|IsEmpty (Variables|/Game/FirstPerson/Blueprints/BP_FirstPersonCharacter.BP_FirstPersonCharacter_C|Getinventory (Variables|Default|GetFPC))))
    (Default|HideInventoryWidget _hud)
    (Default|ShowInteractiveInventoryWidget _hud self)
    (bind _asbp_first_person_game_mode (Utilities|Casting|CastToBP_FirstPersonGameMode (Game|GetGameMode)))
    (Default|PauseGameandShowCursor _asbp_first_person_game_mode)))

(fn ConstructionScript)