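; NPC that plays intro dialogue one second after BeginPlay, plus separate dialogue when the player wins or loses.
; Lines show in a BP_HUD widget, whose Yes button is rebound from advancing to ending on the last line.
; A dialogue-end dispatcher then opens the paused lose menu or calls OnPlayerWin on BP_FirstPersonCharacter.
; Interaction events are empty stubs; helpers play random "no" and laugh sounds.
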(event Custom|AdvanceDialogue
  (bind _hud (Variables|Default|Gethud))
  (bind _dialoguewidgetwithyesbutton (Variables|/Game/UI/HUD/BP_HUD.BP_HUD_C|GetDialogueWidgetWithYesButton _hud))
  (bind _result (Math|Integer|IncrementInt (Variables|Default|GetcurrentDialogueIndex))
    (:%20%20
      (if (>= _result (- (Utilities|Array|Length (Variables|Default|GetcurrentDialogues)) 1))
        (CallFunction|DisplayCurrentDialogue)
        (EventDispatchers|UnbindallEventsfromOnYesButtonClicked _dialoguewidgetwithyesbutton)
        (EventDispatchers|BindEventtoOnYesButtonClicked _dialoguewidgetwithyesbutton (delegate Custom|EndDialogue))
        (else
          (CallFunction|DisplayCurrentDialogue))))))

(event Custom|EndDialogue
  (Default|HideNPCDialoguewithYesButton (Variables|Default|Gethud))
  (Variables|Default|SetisDialogueOngoing false)
  (Default|CallOnDialogueEnd))

(event Custom|OnPlayerLose
  (Variables|Default|SetcurrentDialogueIndex -1)
  (Utilities|Array|Clear (Variables|Default|GetcurrentDialogues))
  (Variables|Default|SetcurrentDialogues (Variables|Default|GetplayerLoseDialogues))
  (CallFunction|BeginInteraction)
  (EventDispatchers|UnbindallEventsfromOnDialogueEnd)
  (EventDispatchers|BindEventtoOnDialogueEnd (delegate Custom|AfterPlayerLoseDialogue)))

(event Custom|BeginInteraction
  (bind _hud (Variables|Default|Gethud))
  (bind _dialoguewidgetwithyesbutton (Variables|/Game/UI/HUD/BP_HUD.BP_HUD_C|GetDialogueWidgetWithYesButton _hud))
  (Variables|Default|SetisDialogueOngoing true)
  (if (not (>= (Variables|Default|GetcurrentDialogueIndex) (- (Utilities|Array|Length (Variables|Default|GetcurrentDialogues)) 1)))
    (EventDispatchers|UnbindallEventsfromOnYesButtonClicked _dialoguewidgetwithyesbutton)
    (EventDispatchers|BindEventtoOnYesButtonClicked _dialoguewidgetwithyesbutton (delegate Custom|AdvanceDialogue))
    (CallFunction|AdvanceDialogue)))

(event Custom|OnPlayerWin
  (Development|PrintString "bp npc on player win")
  (Variables|Default|SetcurrentDialogueIndex -1)
  (Utilities|Array|Clear (Variables|Default|GetcurrentDialogues))
  (Variables|Default|SetcurrentDialogues (Variables|Default|GetplayerwinDialogues))
  (CallFunction|BeginInteraction)
  (EventDispatchers|UnbindallEventsfromOnDialogueEnd)
  (EventDispatchers|BindEventtoOnDialogueEnd (delegate Custom|AfterPlayerWinDialogue)))

(event Custom|AfterPlayerLoseDialogue
  (bind _asbp_first_person_game_mode (Utilities|Casting|CastToBP_FirstPersonGameMode (Game|GetGameMode)))
  (Default|PauseGameandShowCursor _asbp_first_person_game_mode)
  (Default|ShowLevelEndMenu (Variables|Default|Gethud) "Bummer, you lost"))

(event Custom|AfterPlayerWinDialogue
  (bind _returnvalue (Actor|GetActorOfClass "/Game/FirstPerson/Blueprints/BP_FirstPersonCharacter.BP_FirstPersonCharacter_C"))
  (Default|OnPlayerWin _returnvalue))

(event EventBeginPlay
  (bind _returnvalue (Actor|GetActorOfClass "/Game/UI/HUD/BP_HUD.BP_HUD_C"))
  (Variables|Default|Sethud _returnvalue)
  (Variables|Default|SetcurrentDialogues (Variables|Default|GetintroDialogues))
  (Variables|Default|SetcurrentDialogueIndex -1)
  (Utilities|FlowControl|Delay 1.0)
  (CallFunction|BeginInteraction))

(event Collision|EventActorBeginOverlap
  (params (OtherActor :type Actor%20Object%20Reference)))

(event EventTick
  (params (DeltaSeconds :type Float%20%28single-precision%29)))

(event EventDisplayInteractMsg)

(event EventInteract)

(fn ConstructionScript)

(fn DisplayCurrentDialogue
  (Default|DisplayNPCDialoguewithYesButton (Variables|Default|Gethud) (Utilities|Array|Get(acopy) (Variables|Default|GetcurrentDialogues) (Variables|Default|GetcurrentDialogueIndex))))

(fn PlayNoSound
  (Audio|PlaySound2D (Utilities|Array|Get(acopy) (Variables|Default|GetnoSounds) (Math|Random|RandomIntegerinRange 0 (- (Utilities|Array|Length (Variables|Default|GetnoSounds)) 1))) 2.0 1.0 0.0 0 0))

(fn PlayLaughSound
  (Audio|PlaySound2D (Utilities|Array|Get(acopy) (Variables|Default|GetlaughSounds) (Math|Random|RandomIntegerinRange 0 (- (Utilities|Array|Length (Variables|Default|GetlaughSounds)) 1))) 2.0 1.0 0.0 0 0))