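; BP_Moon is an interactable moon punchline item that the player can collect into their inventory once.
; While it is uncollected, it shows a HUD raycast prompt to click a picture of the moon.
; Interacting passes its ItemInfo to the first-person character's AddItemToInventory and sets IsInteracted only on success.
; The actor stays in the world afterwards, as the debug print and DestroyActor nodes are disconnected.
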(event EventBeginPlay)

(event Collision|EventActorBeginOverlap
  (params (OtherActor :type Actor%20Object%20Reference)))

(event EventTick
  (params (DeltaSeconds :type Float%20%28single-precision%29)))

(event EventInteract
  (if (not (Variables|Default|GetisInteracted))
    (bind _returnvalue (Actor|GetActorOfClass "/Game/FirstPerson/Blueprints/BP_FirstPersonCharacter.BP_FirstPersonCharacter_C"))
    (bind _wasitemadded (Default|AddItemtoInventory _returnvalue (Variables|Default|GetitemInfo)))
    (if _wasitemadded
      (Variables|Default|SetisInteracted true))))

(event EventDisplayInteractMsg
  (if (not (Variables|Default|GetisInteracted))
    (Default|DisplayRaycastMsg (Variables|Default|Gethud) "Click a picture of the moon")))

(fn ConstructionScript)