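; BP_Tutor is a tutorial NPC that shows a "Talk" prompt and steps through a list of dialogue lines when interacted with.
; It finds BP_HUD on BeginPlay and displays lines through its dialogue widget with a Yes button.
; The Yes button is bound to advance the dialogue, then rebound on the final line to hide it.
; Once the index reaches the last line, further interaction does nothing.
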(event Custom|AdvanceDialogue
  (bind _hud (Variables|Default|Gethud))
  (bind _dialoguewidgetwithyesbutton (Variables|/Game/UI/HUD/BP_HUD.BP_HUD_C|GetDialogueWidgetWithYesButton _hud))
  (bind _result (Math|Integer|IncrementInt (Variables|Default|GetcurrentDialogueIndex))
    (:%20%20
      (if (>= _result (- (Utilities|Array|Length (Variables|Default|GettutorialDialogues)) 1))
        (CallFunction|DisplayCurrentDialogue)
        (EventDispatchers|UnbindallEventsfromOnYesButtonClicked _dialoguewidgetwithyesbutton)
        (EventDispatchers|BindEventtoOnYesButtonClicked _dialoguewidgetwithyesbutton (delegate Custom|EndDialogue))
        (else
          (CallFunction|DisplayCurrentDialogue))))))

(event Custom|EndDialogue
  (Default|HideNPCDialoguewithYesButton (Variables|Default|Gethud)))

(event EventBeginPlay
  (bind _returnvalue (Actor|GetActorOfClass "/Game/UI/HUD/BP_HUD.BP_HUD_C"))
  (Variables|Default|Sethud _returnvalue))

(event Collision|EventActorBeginOverlap
  (params (OtherActor :type Actor%20Object%20Reference)))

(event EventTick
  (params (DeltaSeconds :type Float%20%28single-precision%29)))

(event EventDisplayInteractMsg
  (Default|DisplayRaycastMsg (Variables|Default|Gethud) "Talk"))

(event EventInteract
  (bind _hud (Variables|Default|Gethud))
  (bind _dialoguewidgetwithyesbutton (Variables|/Game/UI/HUD/BP_HUD.BP_HUD_C|GetDialogueWidgetWithYesButton _hud))
  (if (not (>= (Variables|Default|GetcurrentDialogueIndex) (- (Utilities|Array|Length (Variables|Default|GettutorialDialogues)) 1)))
    (EventDispatchers|UnbindallEventsfromOnYesButtonClicked _dialoguewidgetwithyesbutton)
    (EventDispatchers|BindEventtoOnYesButtonClicked _dialoguewidgetwithyesbutton (delegate Custom|AdvanceDialogue))
    (CallFunction|AdvanceDialogue)))

(fn ConstructionScript)

(fn DisplayCurrentDialogue
  (Default|DisplayNPCDialoguewithYesButton (Variables|Default|Gethud) (Utilities|Array|Get(acopy) (Variables|Default|GettutorialDialogues) (Variables|Default|GetcurrentDialogueIndex))))